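; BP_MenuHUD is the menu HUD for BimodularBot, displaying the WBP_Menu widget and providing travel into the game world.
; BeginPlay creates the widget for the owning player and adds it to that player's screen.
; The construction script also constructs one and adds it to the viewport, so BeginPlay overwrites the MenuWidget reference.
; TravelToGameWorld calls TravelToDemoLevel on BP_BBGameInstance, a placeholder until a non-demo level replaces it.
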(event `self.ReceiveBeginPlay`
  (bind _returnvalue (`|CreateWidget` "/Game/BimodularBot/Menu/UI/WBP_Menu.WBP_Menu_C" (`self.PlayerOwner`)))
  (bind _output_get (set `self.MenuWidget` _returnvalue))
  (`UserWidget.AddToPlayerScreen` _output_get 0))

(fn `TravelToGameWorld`
  ; TODO change this to non demo level
  (bind _asbp_bbgame_instance (cast `/Game/BimodularBot/Core/BP_BBGameInstance` (`GameplayStatics.GetGameInstance`)))
  (`/Game/BimodularBot/Core/BP_BBGameInstance.TravelToDemoLevel` _asbp_bbgame_instance))

(fn `UserConstructionScript`
  (bind _returnvalue (`|GenericCreateObject` "/Game/BimodularBot/Menu/UI/WBP_Menu.WBP_Menu_C"))
  (bind _output_get (set `self.MenuWidget` _returnvalue))
  (`UserWidget.AddToViewport` _output_get 0))