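; Lower-half character of the Bimodular Bot, which merges with and splits from the upper character controlled by the second player.
; On merge, it sets itself as the upper character's TargetActor, grows its capsule, shifts its mesh down and switches the spring arm to the merged camera distance.
; On split, it clears that target and reverses those changes.
; Both handlers run the parent logic first and stop if the second player's pawn is not BP_BBUpperCharacter.
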(event `self.OnMerge`
  (`parent.OnMerge`)
  (bind _secondplayercontroller (`/Game/BimodularBot/Core/BP_BBUtils_Macros.GetSecondPlayer`))
  (bind _asbp_bbupper_character (cast `/Game/BimodularBot/Core/BP_BBUpperCharacter` (`Controller.K2_GetPawn` _secondplayercontroller)))
  ; SetToValue
  (set `/Game/BimodularBot/Core/BP_BBUpperCharacter.TargetActor` self _asbp_bbupper_character)
  (`CapsuleComponent.SetCapsuleHalfHeight` (`self.CapsuleComponent`) 330.0 true)
  (`SceneComponent.K2_AddLocalOffset` (`self.Mesh`) (0.0 0.0 -180.0) false false)
  (set `SpringArmComponent.TargetArmLength` (`self.MergedCameraDistance`) (`self.CameraSpringArm`)))

(event `self.OnSplit`
  (`parent.OnSplit`)
  (bind _secondplayercontroller (`/Game/BimodularBot/Core/BP_BBUtils_Macros.GetSecondPlayer`))
  (bind _asbp_bbupper_character (cast `/Game/BimodularBot/Core/BP_BBUpperCharacter` (`Controller.K2_GetPawn` _secondplayercontroller)))
  ; SetToNull
  (set `/Game/BimodularBot/Core/BP_BBUpperCharacter.TargetActor` null _asbp_bbupper_character)
  (`CapsuleComponent.SetCapsuleHalfHeight` (`self.CapsuleComponent`) 150.0 true)
  (`SceneComponent.K2_AddLocalOffset` (`self.Mesh`) (0.0 0.0 180.0) false false)
  (set `SpringArmComponent.TargetArmLength` (`self.DefaultCameraDistance`) (`self.CameraSpringArm`)))

(fn `UserConstructionScript`
  (`parent.UserConstructionScript`))