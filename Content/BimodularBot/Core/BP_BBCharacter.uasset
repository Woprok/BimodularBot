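; BP_BBCharacter is the Bimodular Bot character Blueprint, handling a debug-press interaction for opening button-linked doors and counting batteries.
; Overlap events on its Box component toggle a ReadyToInteract flag.
; When the flag is set, the press marks overlapping Button actors as pressed and destroys each one's DoorToOpen actor.
; Otherwise, the press increments and prints BatteriesCollected without checking for any battery.
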(event `self.OnDebugPressed_BP`
  (if (`self.ReadyToInteract`)
    (for _array_element (`self.GetOverlappingActors` "/Game/BimodularBot/Maps/Dev/Zuzka/Button.Button_C")
      (set `/Game/BimodularBot/Maps/Dev/Zuzka/Button.Pressed` true _array_element)
      (bind _asbutton (cast `/Game/BimodularBot/Maps/Dev/Zuzka/Button` _array_element))
      (if (`/Game/BimodularBot/Maps/Dev/Zuzka/Button.Pressed` _asbutton)
        (`self.K2_DestroyActor` (`/Game/BimodularBot/Maps/Dev/Zuzka/Button.DoorToOpen` _asbutton))
        (`KismetSystemLibrary.PrintString` "Button pressed, door opened")))
    (else
      (`KismetSystemLibrary.PrintString` "Picked battery. Batteries collected: ")
      (`/Engine/EditorBlueprintResources/StandardMacros.IncrementInt` (`self.BatteriesCollected`)
        (:`  `
          (`KismetSystemLibrary.PrintString` (`KismetStringLibrary.Conv_IntToString` (`self.BatteriesCollected`))))))))

(event `self.Box.OnComponentBeginOverlap`
  (params (OverlappedComponent :type "PrimitiveComponent Object Reference") (OtherActor :type "Actor Object Reference") (OtherComp :type "PrimitiveComponent Object Reference") (OtherBodyIndex :type Integer) (bFromSweep :type Boolean) (SweepResult :type "HitResult Structure (by ref)"))
  (set `self.ReadyToInteract` true))

(event `self.Box.OnComponentEndOverlap`
  (params (OverlappedComponent :type "PrimitiveComponent Object Reference") (OtherActor :type "Actor Object Reference") (OtherComp :type "PrimitiveComponent Object Reference") (OtherBodyIndex :type Integer))
  (set `self.ReadyToInteract` false))

(fn `UserConstructionScript`)