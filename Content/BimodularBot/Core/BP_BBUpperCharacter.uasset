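; BP_BBUpperCharacter is the upper character of the bimodular bot, handling merge and split with its counterpart.
; Merging disables capsule collision and forces splitscreen off.
; Splitting restores both and places the character just ahead of player 0's pawn on the horizontal plane.
; Every tick, while TargetActor is valid, it copies that actor's rotation and its location plus TargetOffset, following by transform rather than attachment.
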(event `self.OnMerge`
  (`parent.OnMerge`)
  (`PrimitiveComponent.SetCollisionProfileName` (`self.CapsuleComponent`) (`self.NoCollision`) true)
  (`GameplayStatics.SetForceDisableSplitscreen` true))

(event `self.OnSplit`
  (bind _returnvalue (`GameplayStatics.GetPlayerPawn` 0))
  (`parent.OnSplit`)
  (`self.K2_SetActorLocation` (+ (`self.K2_GetActorLocation` _returnvalue) (* (`self.GetActorForwardVector` _returnvalue) (50.0 50.0 0.0))))
  (`PrimitiveComponent.SetCollisionProfileName` (`self.CapsuleComponent`) (`self.YesCollision`) true)
  (`GameplayStatics.SetForceDisableSplitscreen` false))

(event `self.ReceiveTick`
  (params (DeltaSeconds :type "Float (single-precision)"))
  (bind _targetactor (`self.TargetActor`))
  (`parent.ReceiveTick` DeltaSeconds)
  (`/Engine/EditorBlueprintResources/StandardMacros.IsValid` _targetactor
    (:`Is Valid`
      (`self.K2_SetActorLocation` (+ (`self.K2_GetActorLocation` _targetactor) (`self.TargetOffset`)))
      (`self.K2_SetActorRotation` (`self.K2_GetActorRotation` _targetactor)))))

(fn `UserConstructionScript`
  (`parent.UserConstructionScript`))