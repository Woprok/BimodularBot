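; BimodularBot game instance that handles travel between the menu and demo levels and gives access to the two split-screen players.
; Two travel events open MenuLevel and the Env_Zuzka demo level through separate menu-level and game-level open calls.
; GetFirstPlayer and GetSecondPlayer wrap the split-screen player lookups, returning each result cast to BP_BBPlayerController.
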(event `TravelToMenuLevel`
  (`self.OpenMenuLevel` "/Game/BimodularBot/Maps/MenuLevel.MenuLevel"))

(event `TravelToDemoLevel`
  (`self.OpenGameLevel` "/Game/BimodularBot/Maps/Dev/Zuzka/Env_Zuzka.Env_Zuzka"))

(fn `GetFirstPlayer`
  (returns (FirstPlayerController :type "/Game/BimodularBot/Core/BP_BBPlayerController Object Reference"))
  (bind _returnvalue (`self.GetFirstSplitscreenPlayer`))
  (bind _asbp_bbplayer_controller (cast `/Game/BimodularBot/Core/BP_BBPlayerController` _returnvalue))
  (return _asbp_bbplayer_controller))

(fn `GetSecondPlayer`
  (returns (SecondPlayerController :type "/Game/BimodularBot/Core/BP_BBPlayerController Object Reference"))
  (bind _returnvalue (`self.GetSecondSplitscreenPlayer`))
  (bind _asbp_bbplayer_controller (cast `/Game/BimodularBot/Core/BP_BBPlayerController` _returnvalue))
  (return _asbp_bbplayer_controller))