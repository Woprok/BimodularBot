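; Dev-map door Blueprint that slides the Door component along its relative Z axis when its Open event is called.
; Open toggles on IsOpen, using one timeline played from start to open and a separate timeline reversed from end to close, with debug prints.
; The flag updates during timeline playback.
; Overlap events only cast to Character and trigger nothing, so Open has no caller in this Blueprint.
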(event `/Game/BimodularBot/Maps/Dev/Zuzka/BP_BI_Openable.Open`
  (if (`self.IsOpen`)
    (`KismetSystemLibrary.PrintString` "Goodbye")
    (bind (_direction _doormovement) (`Timeline|DoorMovemenr` :!via `ReverseFromEnd`)
      (:`Update`
        (`SceneComponent.K2_SetRelativeLocation` (`self.Door`) (`KismetMathLibrary.MakeVector` 0.0 0.0 _doormovement) false false)
        (set `self.IsOpen` false)))
    (else
      (`KismetSystemLibrary.PrintString` "Hello")
      (bind (_direction_2 _doormovement_2) (`Timeline|Timeline` :!via `PlayFromStart`)
        (:`Update`
          (`SceneComponent.K2_SetRelativeLocation` (`self.Door`) (`KismetMathLibrary.MakeVector` 0.0 0.0 _doormovement_2) false false)
          (set `self.IsOpen` true))))))

(event `self.Door.OnComponentBeginOverlap`
  (params (OverlappedComponent :type "PrimitiveComponent Object Reference") (OtherActor :type "Actor Object Reference") (OtherComp :type "PrimitiveComponent Object Reference") (OtherBodyIndex :type Integer) (bFromSweep :type Boolean) (SweepResult :type "HitResult Structure (by ref)"))
  (cast `Character` OtherActor))

(event `self.Door.OnComponentEndOverlap`
  (params (OverlappedComponent :type "PrimitiveComponent Object Reference") (OtherActor :type "Actor Object Reference") (OtherComp :type "PrimitiveComponent Object Reference") (OtherBodyIndex :type Integer))
  (cast `Character` OtherActor))

(fn `UserConstructionScript`)