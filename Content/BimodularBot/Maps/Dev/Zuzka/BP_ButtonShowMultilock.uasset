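; Indicator Blueprint that shows whether a linked Button is pressed, apparently for a multilock.
; Tick polls the Button, mirrors its state into its own Pressed flag and sets the mesh's second material slot to green or red.
; The construction script creates dynamic material instances from the on and off materials to fill those colour variables.
; Its interaction event is implemented but empty.
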(event `self.InteractMyInteraction`)

(event `self.ReceiveTick`
  (params (DeltaSeconds :type "Float (single-precision)"))
  (if (`/Game/BimodularBot/Maps/Dev/Zuzka/BP_Button.Pressed` (`self.Button`))
    (set `self.Pressed` true)
    (`PrimitiveComponent.SetMaterial` (`self.StaticMesh`) 1 (`self.GreenMaterial`))
    (else
      (set `self.Pressed` false)
      (`PrimitiveComponent.SetMaterial` (`self.StaticMesh`) 1 (`self.RedMaterial`)))))

(fn `UserConstructionScript`
  (`KismetMaterialLibrary.CreateDynamicMaterialInstance` "/Game/BimodularBot/Assets/Materials/vypnute.vypnute")
  (set `self.RedMaterial` "/Game/BimodularBot/Assets/Materials/MI_vypnute.MI_vypnute")
  (`KismetMaterialLibrary.CreateDynamicMaterialInstance` "/Game/BimodularBot/Assets/Materials/zapnute.zapnute")
  (set `self.GreenMaterial` "/Game/BimodularBot/Assets/Materials/MI_zapnute.MI_zapnute"))