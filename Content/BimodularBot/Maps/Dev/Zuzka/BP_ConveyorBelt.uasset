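; Conveyor belt actor that carries any actor overlapping its box along an arrow's axis at a set speed.
; Each Tick it offsets overlapping actors, with sweep for everything except movable crates.
; Crates use a Moved flag so overlapping belt triggers do not push them twice in a frame.
; StartStopMoving reverses the direction rather than stopping the belt, and swaps the arrow material to match.
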(event `self.ReceiveTick`
  (params (DeltaSeconds :type "Float (single-precision)"))
  (bind _returnvalue (* (* DeltaSeconds (`self.Speed`)) (`KismetMathLibrary.GetForwardVector` (`SceneComponent.K2_GetComponentRotation` (`self.Arrow`)))))
  (bind _returnvalue_2 (`KismetMathLibrary.NegateVector` _returnvalue))
  (for _array_element (`PrimitiveComponent.GetOverlappingActors` (`self.Box`) null)
    ; This is fix for movable crete to not move it by all conveyor belt (because of big mesh it was overlapping two triggers) (on crete itself, you need move cube to root and update moved to false every tick)
    (bind _asbp_movable_crate (cast `/Game/BimodularBot/Maps/Dev/Zuzka/BP_MovableCrate` _array_element)
      (:`then`
        (if (not (`/Game/BimodularBot/Maps/Dev/Zuzka/BP_MovableCrate.Moved` _asbp_movable_crate))
          (set `/Game/BimodularBot/Maps/Dev/Zuzka/BP_MovableCrate.Moved` true _asbp_movable_crate)
          (if (`self.TurnedOnCorrectly`)
            (`self.K2_AddActorWorldOffset` _array_element _returnvalue_2 false false)
            (else
              (`KismetSystemLibrary.PrintString` (`KismetSystemLibrary.GetDisplayName` _array_element))
              (`self.K2_AddActorWorldOffset` _array_element _returnvalue false false)))))
      (:`CastFailed`
        (if (`self.TurnedOnCorrectly`)
          (`self.K2_AddActorWorldOffset` _array_element _returnvalue_2 true false)
          (else
            (`self.K2_AddActorWorldOffset` _array_element _returnvalue true false)))))))

(event `/Game/BimodularBot/Maps/Dev/Zuzka/BP_BI_StartStopMoving.StartStopMoving`
  (if (`self.TurnedOnCorrectly`)
    (set `self.TurnedOnCorrectly` false)
    (`PrimitiveComponent.SetMaterial` (`self.StaticMesh2`) 0 (`self.MaterialMovingBackward`))
    (else
      (set `self.TurnedOnCorrectly` true)
      (`PrimitiveComponent.SetMaterial` (`self.StaticMesh2`) 0 (`self.MaterialMoving`)))))

(fn `UserConstructionScript`
  (`KismetMaterialLibrary.CreateDynamicMaterialInstance` "/Game/BimodularBot/Maps/Dev/Zuzka/MI_ArrowBackwardMoving.MI_ArrowBackwardMoving")
  (set `self.MaterialMovingBackward` "/Game/BimodularBot/Maps/Dev/Zuzka/MI_ArrowBackwardMoving.MI_ArrowBackwardMoving")
  (`KismetMaterialLibrary.CreateDynamicMaterialInstance` "/Game/BimodularBot/Maps/Dev/Zuzka/MI_ArrowMoving.MI_ArrowMoving")
  (set `self.MaterialMoving` "/Game/BimodularBot/Maps/Dev/Zuzka/MI_ArrowMoving.MI_ArrowMoving"))