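; BP_Button is a toggle button in a dev map that controls an assigned door through interaction or projectile hits.
; Each interaction flips Pressed, swaps the mesh's second material between red and green, and sends OpenMessage to DoorToOpen in either state.
; Box overlaps trigger it only for MyProjectile's mesh component, a workaround for double triggering from its sphere component.
; The construction script sets up both state materials.
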(event `/Game/BimodularBot/Maps/Dev/Zuzka/BP_BI_Interactable.InteractMyInteraction`
  (if (`self.Pressed`)
    (set `self.Pressed` false)
    (`PrimitiveComponent.SetMaterial` (`self.StaticMesh`) 1 (`self.RedMaterial`))
    (message `/Game/BimodularBot/Maps/Dev/Zuzka/BP_BI_Openable.Open` (`self.DoorToOpen`))
    (else
      (set `self.Pressed` true)
      (`PrimitiveComponent.SetMaterial` (`self.StaticMesh`) 1 (`self.GreenMaterial`))
      (message `/Game/BimodularBot/Maps/Dev/Zuzka/BP_BI_Openable.Open` (`self.DoorToOpen`)))))

(event `self.Box.OnComponentBeginOverlap`
  (params (OverlappedComponent :type "PrimitiveComponent Object Reference") (OtherActor :type "Actor Object Reference") (OtherComp :type "PrimitiveComponent Object Reference") (OtherBodyIndex :type Integer) (bFromSweep :type Boolean) (SweepResult :type "HitResult Structure (by ref)"))
  ; I dont know why it is triggering two times, once for SphereComponent and second time for MeshComponent.. so there is fast ix
  (cast `/Game/MyProjectile` OtherActor)
  (cast `MeshComponent` OtherComp)
  (`self.InteractMyInteraction`))

(fn `UserConstructionScript`
  (`KismetMaterialLibrary.CreateDynamicMaterialInstance` "/Game/BimodularBot/Assets/Meshes/vypnute.vypnute")
  (set `self.RedMaterial` "/Game/BimodularBot/Assets/Meshes/MI_vypnute.MI_vypnute")
  (`KismetMaterialLibrary.CreateDynamicMaterialInstance` "/Game/BimodularBot/Assets/Meshes/zapnute.zapnute")
  (set `self.GreenMaterial` "/Game/BimodularBot/Assets/Meshes/MI_zapnute.MI_zapnute"))