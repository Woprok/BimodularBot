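; Example multi-lock door controller that opens a door when a switch and a button are both pressed within a time window.
; The first StartTimer call arms a countdown, and later calls during it check both inputs before stopping it and messaging the door to open.
; Tick runs the countdown with debug printing.
; On expiry, it forces both inputs' pressed flags true and triggers their interactions to restore them.
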(event `self.ReceiveTick`
  (params (DeltaSeconds :type "Float (single-precision)"))
  (if (`self.Start`)
    (`self.RemoveElapsedTime` DeltaSeconds)))

(fn `Open`
  (bind _door (`self.Door`))
  (set `self.Start` false)
  (set `/Game/BimodularBot/Maps/Dev/Zuzka/BP_Door.IsOpen` false _door)
  (message `/Game/BimodularBot/Maps/Dev/Zuzka/BP_BI_Openable.Open` _door))

(fn `RemoveElapsedTime`
  (params (ElapsedTime :type "Float (double-precision)"))
  (bind _output_get (set `self.ActualTime` (- (`self.ActualTime`) ElapsedTime)))
  (`KismetSystemLibrary.PrintString` (`KismetStringLibrary.Conv_DoubleToString` _output_get))
  (if (< _output_get 0.0)
    (`self.RestoreSwitches`)))

(fn `RestoreSwitches`
  (bind _switch1 (`self.Switch1`))
  (bind _button1 (`self.Button1`))
  (set `/Game/BimodularBot/Maps/Dev/Zuzka/BP_ControlPanel.Presssed` true _switch1)
  (`/Game/BimodularBot/Maps/Dev/Zuzka/BP_BI_Interactable.InteractMyInteraction` _switch1)
  (set `/Game/BimodularBot/Maps/Dev/Zuzka/BP_Button.Pressed` true _button1)
  (`/Game/BimodularBot/Maps/Dev/Zuzka/BP_BI_Interactable.InteractMyInteraction` _button1)
  (set `self.Start` false))

(fn `StartTimer`
  (if (`self.Start`)
    (if (`/Game/BimodularBot/Maps/Dev/Zuzka/BP_ControlPanel.Presssed` (`self.Switch1`))
      (if (`/Game/BimodularBot/Maps/Dev/Zuzka/BP_Button.Pressed` (`self.Button1`))
        (`self.Open`)))
    (else
      (set `self.ActualTime` (`self.Timer`))
      (set `self.Start` true))))

(fn `UserConstructionScript`)