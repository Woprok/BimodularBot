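; BP_MultiLock2PressurePlates is a lock that opens a linked door only while two pressure plates are pressed at the same time.
; Tick polls both buttons, calling Open when both are pressed and Close once either releases, with a Completed flag limiting calls to state changes.
; Both functions set the door's IsOpen to the opposite of their name before calling OpenMessage, which suggests that message toggles the door.
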(event `self.ReceiveTick`
  (params (DeltaSeconds :type "Float (single-precision)"))
  (if (`self.Completed`)
    (if (`/Game/BimodularBot/Maps/Dev/Zuzka/BP_Button.Pressed` (`self.Button1`))
      (if (not (`/Game/BimodularBot/Maps/Dev/Zuzka/BP_Button.Pressed` (`self.Button2`)))
        (`self.Close`))
      (else
        (`self.Close`)))
    (elif (`/Game/BimodularBot/Maps/Dev/Zuzka/BP_Button.Pressed` (`self.Button1`))
      (if (`/Game/BimodularBot/Maps/Dev/Zuzka/BP_Button.Pressed` (`self.Button2`))
        (`self.Open`)))))

(fn `Close`
  (bind _door (`self.Door`))
  (set `self.Completed` false)
  (set `/Game/BimodularBot/Maps/Dev/Zuzka/BP_Door.IsOpen` true _door)
  (message `/Game/BimodularBot/Maps/Dev/Zuzka/BP_BI_Openable.Open` _door))

(fn `Open`
  (bind _door (`self.Door`))
  (set `self.Completed` true)
  (set `/Game/BimodularBot/Maps/Dev/Zuzka/BP_Door.IsOpen` false _door)
  (message `/Game/BimodularBot/Maps/Dev/Zuzka/BP_BI_Openable.Open` _door))

(fn `UserConstructionScript`)