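; Destructible crate actor that breaks apart when a MyProjectile overlaps its Box1 trigger.
; A one-time guard removes the intact Cube mesh, then reveals a physics-simulated GeometryCollection in its place.
; A downward impulse at the Box bounds origin pushes the pieces, and the actor destroys itself after a configurable delay.
; The Destroy event is empty, and a debug "Hello" print remains in the break logic.
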(event `OnCustomDestroy`
  (bind _cube (`self.Cube`))
  (bind _geometrycollection (`self.GeometryCollection`))
  (if (not (`self.IsDestroyed`))
    (set `self.IsDestroyed` true)
    (`SceneComponent.SetVisibility` _cube false false)
    (`PrimitiveComponent.SetSimulatePhysics` _cube false)
    (`PrimitiveComponent.SetEnableGravity` _cube false)
    (`ActorComponent.K2_DestroyComponent` _cube)
    (`KismetSystemLibrary.PrintString` "Hello")
    (`SceneComponent.SetVisibility` _geometrycollection true false)
    (`PrimitiveComponent.SetSimulatePhysics` _geometrycollection true)
    (`PrimitiveComponent.SetEnableGravity` _geometrycollection true)
    (`PrimitiveComponent.AddImpulseAtLocation` (`self.GeometryCollection`) (0.0 0.0 -1000.0) (`KismetSystemLibrary.GetComponentBounds` (`self.Box`)) "None")
    (`KismetSystemLibrary.Delay` (`self.Time`))
    (`self.K2_DestroyActor`)))

(event `/Game/BimodularBot/Maps/Dev/Zuzka/BP_BI_Destructible.Destroy`)

(event `self.Box1.OnComponentBeginOverlap`
  (params (OverlappedComponent :type "PrimitiveComponent Object Reference") (OtherActor :type "Actor Object Reference") (OtherComp :type "PrimitiveComponent Object Reference") (OtherBodyIndex :type Integer) (bFromSweep :type Boolean) (SweepResult :type "HitResult Structure (by ref)"))
  (cast `/Game/MyProjectile` OtherActor)
  (`self.OnCustomDestroy`))

(fn `UserConstructionScript`)