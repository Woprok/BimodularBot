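; BP_TextTimer is an actor that shows a countdown as text in the level through a TextRender component.
; The construction script applies the Text and Color variables to that component.
; Each CountDownEvent call subtracts one frame's delta from CountDown, clamps it at zero and displays the formatted time.
; It has no active tick of its own, the TimerValue input is unused and StopCountdown is empty.
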(event `CountDownEvent`
  (params (TimerValue :type "Float (double-precision)"))
  (bind _output_get (set `self.CountDown` (`KismetMathLibrary.FClamp` (- (`self.CountDown`) (`GameplayStatics.GetWorldDeltaSeconds`)) 0.0 (`self.CountDown`))))
  (`TextRenderComponent.K2_SetText` (`self.TextRender`) (`KismetTextLibrary.Conv_StringToText` (`KismetStringLibrary.TimeSecondsToString` _output_get))))

(event `StopCountdown`)

(fn `UserConstructionScript`
  (`TextRenderComponent.K2_SetText` (`self.TextRender`) (`self.Text`))
  (`TextRenderComponent.SetTextRenderColor` (`self.TextRender`) (`self.Color`)))