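; Control panel on a crate that toggles linked conveyor belts on and off through interaction or a projectile hit.
; Each toggle swaps the on/off panel meshes and sends a start/stop message to every belt in ConveyorBelts.
; Switching on also starts the timer of an optional MultilockObject.
; The box overlap accepts only the projectile's MeshComponent, a quick fix for double triggering from its sphere component.
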(event `self.InteractMyInteraction`
  (bind _multilockobject (`self.MultilockObject`))
  (`KismetSystemLibrary.PrintString` "Conveyor")
  (if (`self.Presssed`)
    (set `self.Presssed` false)
    (`SceneComponent.SetVisibility` (`self.OfPanel`) true false)
    (`SceneComponent.SetVisibility` (`self.OnPanel`) false false)
    (for _array_element (`self.ConveyorBelts`)
      (message `/Game/BimodularBot/Maps/Dev/Zuzka/BP_BI_StartStopMoving.StartStopMoving` _array_element))
    (else
      (set `self.Presssed` true)
      (`SceneComponent.SetVisibility` (`self.OnPanel`) true false)
      (`SceneComponent.SetVisibility` (`self.OfPanel`) false false)
      (for _array_element_2 (`self.ConveyorBelts`)
        (message `/Game/BimodularBot/Maps/Dev/Zuzka/BP_BI_StartStopMoving.StartStopMoving` _array_element_2))
      (if (`KismetSystemLibrary.IsValid` _multilockobject)
        (`/Game/BimodularBot/Maps/Dev/Zuzka/BP_MultiLockDoorExample.StartTimer` _multilockobject)))))

(event `self.Box_0.OnComponentBeginOverlap`
  (params (OverlappedComponent :type "PrimitiveComponent Object Reference") (OtherActor :type "Actor Object Reference") (OtherComp :type "PrimitiveComponent Object Reference") (OtherBodyIndex :type Integer) (bFromSweep :type Boolean) (SweepResult :type "HitResult Structure (by ref)"))
  ; I dont know why it is triggering two times, once for SphereComponent and second time for MeshComponent.. so there is fast ix
  (cast `/Game/MyProjectile` OtherActor)
  (cast `MeshComponent` OtherComp)
  (`self.InteractMyInteraction`))

(fn `UserConstructionScript`
  (set `self.UnpressedMesh` (`self.OfPanel`))
  (set `self.PressedMesh` (`self.OnPanel`))
  (`SceneComponent.SetVisibility` (`self.OnPanel`) false false))