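; BP_PreasurePlate is a pressure plate triggered by projectiles, movable crates and the upper or lower bot characters.
; Box overlap events maintain a Counter of qualifying actors, so only the first arrival and an exit that empties the plate take effect.
; Those changes swap the Cube's on/off material and call the same MyInteraction on the linked Button, or on ControlPanel if no Button is valid.
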(event `self.ReceiveBeginPlay`
  (`PrimitiveComponent.SetMaterial` (`self.Cube`) 1 (`self.MaterailOff`)))

(event `self.Box.OnComponentBeginOverlap`
  (params (OverlappedComponent :type "PrimitiveComponent Object Reference") (OtherActor :type "Actor Object Reference") (OtherComp :type "PrimitiveComponent Object Reference") (OtherBodyIndex :type Integer) (bFromSweep :type Boolean) (SweepResult :type "HitResult Structure (by ref)"))
  (bind _button (`self.Button`))
  (bind _controlpanel (`self.ControlPanel`))
  ; Go throught all possible starter
  (cast `/Game/MyProjectile` OtherActor
    (:`then`
      _)
    (:`CastFailed`
      (cast `/Game/BimodularBot/Maps/Dev/Zuzka/BP_MovableCrate` OtherActor
        (:`then`
          _)
        (:`CastFailed`
          (cast `/Game/BimodularBot/Core/BP_BBLowerCharacter` OtherActor
            (:`then`
              _)
            (:`CastFailed`
              (cast `/Game/BimodularBot/Core/BP_BBUpperCharacter` OtherActor)))))))
  (bind _output_get (set `self.Counter` (+ (`self.Counter`) 1)))
  ; Change color
  (if (== _output_get 1)
    (`PrimitiveComponent.SetMaterial` (`self.Cube`) 1 (`self.MaterailOn`))
    ; Button
    (if (`KismetSystemLibrary.IsValid` _button) :!label _label
      (`KismetSystemLibrary.PrintString` (`KismetSystemLibrary.GetDisplayName` _button))
      (`/Game/BimodularBot/Maps/Dev/Zuzka/BP_BI_Interactable.InteractMyInteraction` _button)
      (else
        ; Pannel
        (if (`KismetSystemLibrary.IsValid` _controlpanel)
          (`KismetSystemLibrary.PrintString` (`KismetSystemLibrary.GetDisplayName` _controlpanel))
          (`/Game/BimodularBot/Maps/Dev/Zuzka/BP_BI_Interactable.InteractMyInteraction` _controlpanel))))))

(event `self.Box.OnComponentEndOverlap`
  (params (OverlappedComponent :type "PrimitiveComponent Object Reference") (OtherActor :type "Actor Object Reference") (OtherComp :type "PrimitiveComponent Object Reference") (OtherBodyIndex :type Integer))
  ; Go throught all possible starter
  (cast `/Game/MyProjectile` OtherActor
    (:`then`
      _)
    (:`CastFailed`
      (cast `/Game/BimodularBot/Maps/Dev/Zuzka/BP_MovableCrate` OtherActor
        (:`then`
          _)
        (:`CastFailed`
          (cast `/Game/BimodularBot/Core/BP_BBLowerCharacter` OtherActor
            (:`then`
              _)
            (:`CastFailed`
              (cast `/Game/BimodularBot/Core/BP_BBUpperCharacter` OtherActor)))))))
  (bind _output_get (set `self.Counter` (`KismetMathLibrary.Max` 0 (- (`self.Counter`) 1))))
  (if (<= _output_get 0)
    ; Change color
    (`PrimitiveComponent.SetMaterial` (`self.Cube`) 1 (`self.MaterailOff`))
    (goto _label)))

(fn `UserConstructionScript`)