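; BP_DebugCharacter is a developer test actor that moves forward along its local X axis while the move input is active.
; IA_Move events set a Go flag on start, ongoing or trigger and clear it on cancel or completion, ignoring the input's value.
; Tick applies a swept local offset scaled by Speed and delta time while Go is set.
; BeginPlay and every handled input event print a "Hello" debug string.
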(event `self.ReceiveBeginPlay`
  (`KismetSystemLibrary.PrintString` "Hello"))

(event `self.ReceiveTick`
  (params (DeltaSeconds :type "Float (single-precision)"))
  (if (`self.go`)
    (`self.K2_AddActorLocalOffset` (`KismetMathLibrary.MakeVector` (* DeltaSeconds (`self.speed`))) true)))

(event `EnhancedInput|/Game/BimodularBot/Core/Inputs/IA_Move`
  (params (ActionValue :type "Vector2D Structure") (ElapsedSeconds :type "Float (double-precision)") (TriggeredSeconds :type "Float (double-precision)") (InputAction :type "InputAction Object Reference" :default "/Game/BimodularBot/Core/Inputs/IA_Move.IA_Move"))
  (:`Triggered`
    (set `self.go` true :!label _label)
    (`KismetSystemLibrary.PrintString` "Hello" :!label _label_2))
  (:`Started`
    (goto _label))
  (:`Ongoing`
    (goto _label))
  (:`Canceled`
    (set `self.go` false :!label _label_3)
    (goto _label_2))
  (:`Completed`
    (goto _label_3)))

(fn `UserConstructionScript`)